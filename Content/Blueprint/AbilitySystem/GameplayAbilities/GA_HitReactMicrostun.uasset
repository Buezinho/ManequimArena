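; GA_HitReactMicrostun is a gameplay ability that plays a hit reaction on its avatar actor.
; On activation it applies GE_HitReact to the owner, stores the handle, and gets the montage through the avatar's CombatInterface.
; When the montage completes, is interrupted or is cancelled, or if the interface cast fails, it removes that effect and ends the ability.
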(event Ability|EventActivateAbility
  (bind _returnvalue (Ability|ApplyGameplayEffectToOwner "/Game/Blueprint/AbilitySystem/GameplayEffects/GE_HitReact.GE_HitReact_C"))
  (Variables|Default|SetHitReact_Effect _returnvalue)
  (bind _ascombat_interface (Utilities|Casting|CastToCombatInterface (Ability|GetAvatarActorfromActorInfo))
    (:then
      (bind _returnvalue_2 (Class|CombatInterface|GetHitReactMontage _ascombat_interface))
      (|PlayMontageandWaitProxy "None" _returnvalue_2 1.0 "None" true 1.0 0.0 false
        (:OnCompleted
          _)
        (:OnInterrupted
          _)
        (:OnCancelled
          _)))
    (:CastFailed
      _))
  (Ability|RemoveGameplayEffectFromOwnerWithHandle (Variables|Default|GetHitReact_Effect))
  (Ability|EndAbility))

(event Ability|EventOnEndAbility
  (params (bWasCancelled :type Boolean)))